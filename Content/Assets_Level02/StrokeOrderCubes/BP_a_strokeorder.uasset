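; Clickable stroke-order actor for the "a" character that updates matching on-screen text and celebrates when clicked.
; On click, it searches top-level DynamicText widgets for text equal to its CharacterDetector value.
; Each match receives an UpdateLetter call with that text, plays a 2D sound and activates the confetti Niagara effect.
; Confetti is deactivated at BeginPlay, and the box overlap event is empty.
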(event OnComponentBeginOverlap(BoxCollision)
  (params (OverlappedComponent :type Primitive%20Component%20Object%20Reference) (OtherActor :type Actor%20Object%20Reference) (OtherComp :type Primitive%20Component%20Object%20Reference) (OtherBodyIndex :type Integer) (bFromSweep :type Boolean) (SweepResult :type Hit%20Result%20Structure%20%28by%20ref%29)))

(event EventBeginPlay
  (Components|Activation|Deactivate (Variables|Default|GetConfetti%20Niagra)))

(event MouseInput|EventActorOnClicked
  (params (ButtonPressed :type Key%20Structure :default "None"))
  (bind _output_get (Variables|Default|SetIsPressed true))
  (if _output_get
    (bind _foundwidgets (Widget|GetAllWidgetsOfClass "/Game/Assets_Level01/DynamicText.DynamicText_C" true))
    (for _array_element _foundwidgets
      (if (Utilities|Enum|Equal(Enum) (Utilities|String|ToString(Text) (Class|TextBlock|GetText (Variables|/Game/Assets_Level01/DynamicText.DynamicText_C|GetDynamicText _array_element))) (Utilities|String|ToString(Text) (Variables|Default|GetCharacterDetector)))
        (bind _output_get_2 (Variables|Default|SetRandomChecker (Class|TextBlock|GetText (Variables|/Game/Assets_Level01/DynamicText.DynamicText_C|GetDynamicText _array_element))))
        (Default|UpdateLetter _array_element _output_get_2)
        (Audio|PlaySound2D (Variables|Default|GetSoundVariable) 1.0 1.0 0.0 0 0)
        (Components|Activation|Activate (Variables|Default|GetConfetti%20Niagra) false)))))

(fn ConstructionScript)